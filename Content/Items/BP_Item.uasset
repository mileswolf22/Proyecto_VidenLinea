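; BP_Item is a world pickup that the player collects into their inventory with F.
; BeginPlay builds its full info from the Tabla_Items row named by the item enum, keeping the instance's quantity, and passes it to the info widget.
; Character overlap toggles input; pressing F adds the item, destroys the actor and refreshes InventarioWidget.
; ItemSeleccionado toggles custom-depth rendering and widget visibility for selection highlighting.
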(event OnComponentBeginOverlap(Colision)
  (params (OverlappedComponent :type Primitive%20Component%20Object%20Reference) (OtherActor :type Actor%20Object%20Reference) (OtherComp :type Primitive%20Component%20Object%20Reference) (OtherBodyIndex :type Integer) (bFromSweep :type Boolean) (SweepResult :type Hit%20Result%20Structure%20%28by%20ref%29))
  (Utilities|Casting|CastToThirdPersonCharacter OtherActor)
  (Input|EnableInput (Game|GetPlayerController 0))
  (Variables|Default|SetPersonajeCerca true))

(event OnComponentEndOverlap(Colision)
  (params (OverlappedComponent :type Primitive%20Component%20Object%20Reference) (OtherActor :type Actor%20Object%20Reference) (OtherComp :type Primitive%20Component%20Object%20Reference) (OtherBodyIndex :type Integer))
  (Utilities|Casting|CastToThirdPersonCharacter OtherActor)
  (Input|DisableInput (Game|GetPlayerController 0))
  (Variables|Default|SetPersonajeCerca false))

(event EventBeginPlay
  (bind _aswg_información_item (Utilities|Casting|CastToWG_Información_Item (UserInterface|GetUserWidgetObject (Variables|Default|GetWidget))))
  (bind _informacióncompleta (CallFunction|ObtenerInformaciónCompleta (Variables|Default|GetInformación)))
  (bind _output_get (Variables|Default|SetInformaciónCompleta _informacióncompleta))
  (Variables|/Game/UI/WG_Información_Item.WG_Información_Item_C|SetInformación _aswg_información_item _output_get))

(event EventTick
  (params (DeltaSeconds :type Float%20%28single-precision%29)))

(event Input|KeyboardEvents|F
  (params (Key :type Key%20Structure :default "None"))
  (:Pressed
    (bind _asthird_person_character (Utilities|Casting|CastToThirdPersonCharacter (Game|Player|GetPlayerPawn 0)))
    (Default|AgregarItem _asthird_person_character (Variables|Default|GetInformaciónCompleta))
    (Actor|DestroyActor)
    (Default|ConfigurarInventario (Variables|/Game/ThirdPersonBP/Blueprints/ThirdPersonCharacter.ThirdPersonCharacter_C|GetInventarioWidget _asthird_person_character) (Variables|/Game/ThirdPersonBP/Blueprints/ThirdPersonCharacter.ThirdPersonCharacter_C|GetInventario%20-%20Items _asthird_person_character) (Variables|/Game/ThirdPersonBP/Blueprints/ThirdPersonCharacter.ThirdPersonCharacter_C|GetInventario%20-%20IC _asthird_person_character))))

(fn ConstructionScript)

(fn ItemSeleccionado
  (params (Seleccionado :type Boolean))
  (Rendering|SetRenderCustomDepth (Variables|Default|GetModelo) Seleccionado)
  (Rendering|SetVisibility (Variables|Default|GetWidget) Seleccionado false))

(fn ObtenerInformaciónCompleta
  (params (Información :type Estructura%20Item%202%20Structure))
  (bind _returnvalue (Utilities|GetDataTableRow "/Game/Items/Tabla_Items.Tabla_Items" (Utilities|String|StringToName (Utilities|String|EnumtoString (.item Información))))
    (:then
      (return (Utilities|Struct|MakeEstructura_Item_Completa (.item _returnvalue) (.nombre _returnvalue) (.cantidad Información) (.imagen _returnvalue) (.columna _returnvalue) (.posicionado _returnvalue) (.valor _returnvalue))))))